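; Grapple arm tool that fires a hook projectile on a cable and recalls it, with server-authoritative spawning and recall.
; TraceForSurface combines a camera line trace, suggested toss velocity and coarse path prediction to find an endpoint and apex.
; MULTI_Launch derives a quadratic Bezier control point from these, and only authority spawns BP_GrappleProjectile along that curve.
; RepNotifies toggle cable and hook visuals; Reach is an empty stub.
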(fn ConstructionScript)

(fn TraceforSurface
  (params (CamLoc :type Vector) (CamRot :type Rotator) (Hero :type Actor%20Object%20Reference) (ProjectileSpeed :type Float%20%28double-precision%29) (DefaultTraceDistance :type Float%20%28single-precision%29) (TrajectoryLength :type Float%20%28single-precision%29) (Debug_ProjectileRadius :type Float%20%28single-precision%29))
  (LocalVariables|SetFinalTracePoint (+ CamLoc (* (Math|Vector|GetForwardVector CamRot) DefaultTraceDistance)))
  (bind (_outhit _returnvalue) (Collision|LineTraceByChannel CamLoc (LocalVariables|GetFinalTracePoint) "TraceTypeQuery1" false (Utilities|Array|MakeArray Hero) "None"))
  (bind _tossvelocity (Class|GameplayStatics|BlueprintSuggestProjectileVelocity CamLoc (Math|Vector|SelectVector (.ImpactPoint (Collision|BreakHitResult _outhit)) (LocalVariables|GetFinalTracePoint) _returnvalue) ProjectileSpeed 0.0 "DoNotTrace" Debug_ProjectileRadius false false false))
  (bind (_outhit_2 _outpathpositions _outlasttracedestination) (Class|GameplayStatics|BlueprintPredictProjectilePathbyObjectType CamLoc _tossvelocity false Debug_ProjectileRadius (Utilities|Array|MakeArray "ObjectTypeQuery11") false (Utilities|Array|MakeArray Hero) "None" 1e+01 (* (/ 1.0 TrajectoryLength) 2.0) TrajectoryLength))
  (return _outlasttracedestination (Utilities|Array|Get(acopy) _outpathpositions 1)))

(fn OnRepHookFired?
  (CallFunction|UpdateHookVisuals))

(fn OnRepProjectile
  (CallFunction|UpdateHookVisuals))

(fn UpdateHookVisuals
  (bind _cable (Variables|Default|GetCable))
  (bind _hook (Variables|Default|GetHook))
  (bind _cable_2 (Variables|Default|GetCable))
  (if (Variables|Default|GetHookFired?)
    (bind _projectile (Variables|Default|GetProjectile)
      (:then
        (Class|CableComponent|SetAttachEndto _cable_2 _projectile "None" "None")
        (Development|SetHiddeninGame _cable false false)
        (Development|SetHiddeninGame _hook true false))
      (:else))
    (else
      (Class|CableComponent|SetAttachEndto _cable_2 0 "None" "None")
      (Development|SetHiddeninGame _cable true false)
      (Development|SetHiddeninGame _hook false false))))

(event EventLeftToolE
  (CallFunction|Launch))

(event EventLeftToolRightClick
  (CallFunction|Recall))

(event EventLeftToolLeftClick
  (CallFunction|Reach))

(event Custom|Recall
  ;[0.15 0.15 0.15 0.5 50] Recall
  (if (Variables|Default|GetHookFired?)
    (Networking|SwitchHasAuthority
      (:Authority
        (bind _projectile (Variables|Default|GetProjectile)
          (:then
            (Default|StartRecalling _projectile))
          (:else)))
      (:Remote
        (CallFunction|SERVRecall)))))

(event Custom|SERV_Recall
  ;[0.15 0.15 0.15 0.5 50] Recall
  (bind _projectile (Variables|Default|GetProjectile)
    (:then
      (Default|StartRecalling _projectile))
    (:else)))

(event Custom|Launch
  (bind _herocam (Variables|Default|GetHeroCam))
  (bind _returnvalue (Transformation|GetWorldTransform _herocam))
  ;[0.15 0.15 0.15 0.5 50] Launch
  (if (not (Variables|Default|GetHookFired?))
    (Networking|SwitchHasAuthority
      (:Authority
        (bind (_p2 _apex) (CallFunction|TraceforSurface (.location _returnvalue) (.rotation _returnvalue) (Variables|Default|GetHero) (Variables|Default|GetProjectileSpeed) (Variables|Default|GetDefault%20Trace%20Distance) (Variables|Default|GetTrajectory%20Length) 1e+02))
        (CallFunction|MULTILaunch (.rotation _returnvalue) (.location _returnvalue) _p2 _apex (GameState|GetServerWorldTimeSeconds (Game|GetGameState))))
      (:Remote
        (CallFunction|SERVLaunch (.location _returnvalue) (.rotation _returnvalue) (Variables|Default|GetHero))))))

(event Custom|Reach
  ;[0.15 0.15 0.15 0.5 50] Reach
)

(event Custom|SERV_Launch
  (params (CamLoc :type Vector) (CamRot :type Rotator) (Hero :type Actor%20Object%20Reference))
  ;[0.15 0.15 0.15 0.5 50] Launch
  (bind (_p2 _apex) (CallFunction|TraceforSurface CamLoc CamRot Hero (Variables|Default|GetProjectileSpeed) (Variables|Default|GetDefault%20Trace%20Distance) (Variables|Default|GetTrajectory%20Length) 1e+02))
  (CallFunction|MULTILaunch CamRot CamLoc _p2 _apex (GameState|GetServerWorldTimeSeconds (Game|GetGameState))))

(event Custom|MULTI_Launch
  (params (CamRot :type Rotator) (P0 :type Vector) (P2 :type Vector) (Apex :type Vector) (StartTime :type Float%20%28double-precision%29))
  ;[0.15 0.15 0.15 0.5 50] Launch
  (Variables|Default|SetP0 P0)
  (Variables|Default|SetP2 P2)
  (Variables|Default|SetApex Apex)
  (bind _output_get (Variables|Default|SetP1 (- (* (Math|Vector|MakeVector (.X (Math|Vector|BreakVector (* (+ (Variables|Default|GetP0) (Variables|Default|GetP2)) 0.5))) (.Y (Math|Vector|BreakVector (* (+ (Variables|Default|GetP0) (Variables|Default|GetP2)) 0.5))) (.z (Variables|Default|GetApex))) 2.0) (* (+ (Variables|Default|GetP0) (Variables|Default|GetP2)) 0.5))))
  (Networking|SwitchHasAuthority
    (:Authority
      (bind _returnvalue (Game|SpawnActorfromClass "/Game/Weapons/Grapple/Grapple/BP_GrappleProjectile.BP_GrappleProjectile_C" (Math|Transform|MakeTransform (Variables|Default|GetP0) CamRot "1.000000,1.000000,1.000000") "Undefined" "MultiplyWithRoot" self (Variables|Default|GetP0) (Variables|Default|GetP0) (Variables|Default|GetP1) (Variables|Default|GetP2) StartTime (/ (+ (Math|Vector|Distance(Vector) (Variables|Default|GetP0) (Variables|Default|GetP1)) (Math|Vector|Distance(Vector) (Variables|Default|GetP1) (Variables|Default|GetP2))) (Variables|Default|GetProjectileSpeed)) (Variables|Default|GetHero)))
      (Variables|Default|SetProjectile _returnvalue)
      (Variables|Default|SetHookFired? true)
      (CallFunction|UpdateHookVisuals))))