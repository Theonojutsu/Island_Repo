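; Networked grapple hook projectile that launches, sticks to surfaces and recalls to its owning BP_GrappleArm.
; Tick moves it along a curve-eased quadratic Bezier using server world time, line tracing between steps to attach at impacts.
; A miss triggers recall, lerping back to the owner, where the server resets the arm and destroys the hook.
; The server decides hit and recall states; RepNotifies mirror attach and detach on clients.
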(event Custom|StartRecalling
  ;[0.15 0.15 0.15 0.5 50] Recalling
  (Networking|SwitchHasAuthority
    (:Authority
      (Transformation|DetachFromActor "KeepWorld" "KeepWorld" "KeepWorld")
      (Variables|Recall|SetRecallStartTime (GameState|GetServerWorldTimeSeconds (Game|GetGameState)))
      (Variables|Recall|SetRecallStartPos (Transformation|GetActorLocation))
      (Variables|Recall|SetIsRecalling? true)
      (if (not (Class|Actor|IsActorTickEnabled))
        (Actor|Tick|SetActorTickEnabled true)))))

(event EventTick
  (params (DeltaSeconds :type Float%20%28single-precision%29))
  (bind _returnvalue (Game|GetGameState))
  (bind _launchstarttime (Variables|Launch|GetLaunchStartTime))
  (bind _launchduration (Variables|Launch|GetLaunchDuration))
  (bind _returnvalue_2 (GameState|GetServerWorldTimeSeconds _returnvalue))
  (bind _returnvalue_3 (- _returnvalue_2 _launchstarttime))
  (bind _returnvalue_4 (/ _returnvalue_3 _launchduration))
  (bind _returnvalue_5 (Math|Float|Clamp(Float) _returnvalue_4 0.005))
  (if (Variables|Recall|GetIsRecalling?)
    ;[0.15 0.15 0.15 0.5 50] Recalling
    (Transformation|SetActorLocation (Math|Vector|Lerp(Vector) (Variables|Recall|GetRecallStartPos) (Transformation|GetActorLocation (Components|GetOwner)) (Math|Curves|GetFloatValue (Variables|Recall|GetCurveRecall) (Math|Float|Clamp(Float) (/ (* (- (GameState|GetServerWorldTimeSeconds (Game|GetGameState)) (Variables|Recall|GetRecallStartTime)) (Variables|Recall|GetRecallSpeed)) (Math|Vector|Distance(Vector) (Variables|Recall|GetRecallStartPos) (Transformation|GetActorLocation (Components|GetOwner))))))) false false)
    (if (>= (Math|Float|Clamp(Float) (/ (* (- (GameState|GetServerWorldTimeSeconds (Game|GetGameState)) (Variables|Recall|GetRecallStartTime)) (Variables|Recall|GetRecallSpeed)) (Math|Vector|Distance(Vector) (Variables|Recall|GetRecallStartPos) (Transformation|GetActorLocation (Components|GetOwner))))) 1.0)
      (Networking|SwitchHasAuthority
        (:Authority
          (Utilities|FlowControl|Sequence
            (:then_0
              (bind _asbp_grapple_arm (Utilities|Casting|CastToBP_GrappleArm (Components|GetOwner)))
              (Variables|/Game/Weapons/Grapple/Grapple/BP_GrappleArm.BP_GrappleArm_C|SetHookFired? _asbp_grapple_arm false)
              (Variables|/Game/Weapons/Grapple/Grapple/BP_GrappleArm.BP_GrappleArm_C|SetProjectile _asbp_grapple_arm 0)
              (Default|UpdateHookVisuals _asbp_grapple_arm))
            (:then_1
              (Actor|DestroyActor))))))
    (else
      ;[0.15 0.15 0.15 0.5 50] Launching
      (if (> (Variables|Launch|GetLaunchStartTime) 0.0)
        (if (Math|Float|NearlyEqual(Float) _returnvalue_5 1.0 0.05) ; Has reached destination ?
          (Networking|SwitchHasAuthority
            (:Authority
              (Utilities|FlowControl|DoOnce false
                (:Completed
                  (if (not (Variables|Recall|GetIsRecalling?))
                    (Transformation|DetachFromActor "KeepWorld" "KeepWorld" "KeepWorld")
                    (Variables|Recall|SetRecallStartTime (GameState|GetServerWorldTimeSeconds (Game|GetGameState)))
                    (Variables|Recall|SetRecallStartPos (Transformation|GetActorLocation))
                    (Variables|Recall|SetIsRecalling? true)
                    (if (not (Class|Actor|IsActorTickEnabled))
                      (Actor|Tick|SetActorTickEnabled true)))))))
          (else
            (bind _bezpos (CallFunction|GetBezierPos (Variables|Launch|GetP0) (Variables|Launch|GetP1) (Variables|Launch|GetP2) (Math|Curves|GetFloatValue (Variables|Launch|GetCurveLaunch) _returnvalue_5)))
            (Transformation|SetActorLocation _bezpos false false)
            ;[0.15 0.15 0.15 0.5 50] Sticking
            (bind _output_get (Variables|Launch|SetBez%20Pos_Prev (Variables|Launch|GetBez%20Pos)))
            (bind (_outhit _returnvalue_6) (Collision|LineTraceForObjects _output_get _bezpos (Utilities|Array|MakeArray "ObjectTypeQuery1" "ObjectTypeQuery8") false (Utilities|Array|MakeArray (Components|GetOwner) (Variables|Actor|GetInstigator)) "None"))
            (Variables|Launch|SetBez%20Pos _bezpos)
            (if _returnvalue_6
              (Transformation|SetActorLocation (+ (.ImpactPoint (Collision|BreakHitResult _outhit)) (* (Math|Vector|GetUnitDirection(Vector) (Variables|Launch|GetBez%20Pos) (Variables|Launch|GetBez%20Pos_Prev)) (* (.sphereradius (StaticMesh|GetBounds (Variables|/Script/Engine.StaticMeshComponent|GetStaticMesh (Variables|Default|GetHook)))) 2.0 (Math|Float|Clamp(Float) (- 1.0 (/ (Variables|ProjectileParams|GetSurfacePenetration) 1e+02)) 0.01)))) false false)
              (Networking|SwitchHasAuthority
                (:Authority
                  (Actor|Tick|SetActorTickEnabled false)
                  (Transformation|AttachComponentToComponent (.HitComponent (Collision|BreakHitResult _outhit)) "None" "KeepWorld" "KeepWorld" "KeepWorld" true)
                  (Transformation|SetAbsolute (Variables|Default|GetHook) false false true)
                  (Transformation|SetActorScale3D "1.000000,1.000000,1.000000")
                  (Variables|Default|SetHitComponent (.HitComponent (Collision|BreakHitResult _outhit)))
                  (Variables|Launch|SetHitLocation (+ (.ImpactPoint (Collision|BreakHitResult _outhit)) (* (Math|Vector|GetUnitDirection(Vector) (Variables|Launch|GetBez%20Pos) (Variables|Launch|GetBez%20Pos_Prev)) (* (.sphereradius (StaticMesh|GetBounds (Variables|/Script/Engine.StaticMeshComponent|GetStaticMesh (Variables|Default|GetHook)))) 2.0 (Math|Float|Clamp(Float) (- 1.0 (/ (Variables|ProjectileParams|GetSurfacePenetration) 1e+02)) 0.01)))))
                  (Variables|Launch|SetHasHit? true))))))))))

(fn ConstructionScript)

(fn GetBezierPos
  (params (P0 :type Vector) (P1 :type Vector) (P2 :type Vector) (t :type Float%20%28double-precision%29))
  (return (Math|Vector|Lerp(Vector) (Math|Vector|Lerp(Vector) P0 P1 t) (Math|Vector|Lerp(Vector) P1 P2 t) t)))

(fn OnRepIsRecalling?
  (Transformation|DetachFromActor "KeepWorld" "KeepWorld" "KeepWorld")
  (if (not (Class|Actor|IsActorTickEnabled))
    (Actor|Tick|SetActorTickEnabled true)))

(fn OnRepHasHit?
  (if (Variables|Launch|GetHasHit?)
    (Actor|Tick|SetActorTickEnabled false)
    (Transformation|SetActorLocation (Variables|Launch|GetHitLocation) false false)
    (Transformation|AttachComponentToComponent (Variables|Default|GetHitComponent) "None" "KeepWorld" "KeepWorld" "KeepWorld" true)
    (Transformation|SetAbsolute (Variables|Default|GetHook) false false true)
    (Transformation|SetActorScale3D "1.000000,1.000000,1.000000")))