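; BP_LeftTool is a left-hand tool pickup, with empty switch, E and click events as hooks for tool behavior.
; When a BP_HeroBase overlaps PickupZone, the authority attaches the tool if that hero's LeftTool slot is empty.
; Attaching disables pickup collision, snaps the tool to the HandGrip_L mesh socket, caches hero and camera, sets ownership and registers itself as the hero's LeftTool.
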(event OnComponentBeginOverlap(PickupZone)
  (params (OverlappedComponent :type Primitive%20Component%20Object%20Reference) (OtherActor :type Actor%20Object%20Reference) (OtherComp :type Primitive%20Component%20Object%20Reference) (OtherBodyIndex :type Integer) (bFromSweep :type Boolean) (SweepResult :type Hit%20Result%20Structure%20%28by%20ref%29))
  (Networking|SwitchHasAuthority
    (:Authority
      (bind _asbp_hero_base (Utilities|Casting|CastToBP_HeroBase OtherActor))
      (CallFunction|AttachtoPlayer _asbp_hero_base))))

(event Custom|LeftTool_LeftClick)

(event Custom|LeftTool_E)

(event Custom|AttachToPlayer
  (params (Hero :type BP%20Hero%20Base%20Object%20Reference))
  (Variables|/Game/FirstPerson/Blueprints/BP_HeroBase.BP_HeroBase_C|GetLeftTool Hero
    (:then)
    (:else
      (Collision|SetCollisionEnabled (Variables|Default|GetPickupZone) "NoCollision")
      (bind _output_get (Variables|Default|SetHero Hero))
      (Transformation|AttachComponentToComponent self (Variables|/Script/Engine.Character|GetMesh _output_get) "HandGrip_L" "SnapToTarget" "SnapToTarget" "KeepWorld" true)
      (Variables|Default|SetHeroCam (Variables|/Game/FirstPerson/Blueprints/BP_HeroBase.BP_HeroBase_C|GetCamera Hero))
      (Actor|SetOwner (Variables|Default|GetHero))
      (Variables|/Game/FirstPerson/Blueprints/BP_HeroBase.BP_HeroBase_C|SetLeftTool Hero self))))

(event Custom|LeftTool_RightClick)

(event Custom|Switch)

(fn ConstructionScript)