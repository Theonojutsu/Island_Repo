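; BP_Equipable is an equippable pickup that attaches to a hero's HandGrip_L mesh socket when walked over, with empty E, left-click and right-click events.
; On server overlap it disables pickup collision, then scans the hero's attached actors for one of the same class.
; If none matches, it attaches, caches hero and camera, sets its owner and registers itself on the hero.
; Pickup collision stays disabled even when a duplicate blocks equipping.
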(event OnComponentBeginOverlap(PickupZone)
  (params (OverlappedComponent :type Primitive%20Component%20Object%20Reference) (OtherActor :type Actor%20Object%20Reference) (OtherComp :type Primitive%20Component%20Object%20Reference) (OtherBodyIndex :type Integer) (bFromSweep :type Boolean) (SweepResult :type Hit%20Result%20Structure%20%28by%20ref%29))
  (Networking|SwitchHasAuthority
    (:Authority
      (bind _asbp_hero_base (Utilities|Casting|CastToBP_HeroBase OtherActor))
      (Collision|SetCollisionEnabled (Variables|Default|GetPickupZone) "NoCollision")
      (Variables|Default|SetOwned false)
      (bind _array_element (Utilities|Array|ForEachLoopwithBreak (Actor|GetAttachedActors _asbp_hero_base true false) :!label _label)
        (:LoopBody
          (if (Class|GameplayStatics|ObjectIsA _array_element (Utilities|GetClass self))
            (Variables|Default|SetOwned true)
            (goto _label Break)))
        (:Completed
          (if (not (Variables|Default|GetOwned))
            (bind _output_get (Variables|Default|SetHero _asbp_hero_base))
            (Transformation|AttachComponentToComponent self (Variables|/Script/Engine.Character|GetMesh _output_get) "HandGrip_L" "SnapToTarget" "SnapToTarget" "KeepWorld" true)
            (Variables|Default|SetHeroCam (Variables|/Game/FirstPerson/Blueprints/BP_HeroBase.BP_HeroBase_C|GetCamera _asbp_hero_base))
            (Actor|SetOwner (Variables|Default|GetHero))
            (Variables|/Game/FirstPerson/Blueprints/BP_HeroBase.BP_HeroBase_C|SetAs%20BP%20Equipable _asbp_hero_base self)))))))

(event Custom|Equipable_LeftClick)

(event Custom|Equipable_E)

(event Custom|Equipable_RightClick)

(fn ConstructionScript)