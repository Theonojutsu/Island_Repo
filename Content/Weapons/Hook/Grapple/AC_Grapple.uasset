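; Grapple hook component for a Character that attaches an arm actor to the left hand and launches hook projectiles on input.
; The server line-traces from the camera, then uses projectile velocity suggestion and path prediction to derive an end point and apex.
; A multicast turns these into three quadratic Bezier-style control points.
; Each machine spawns its own projectile with those points, a server start time and a distance-based duration.
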(event Custom|MULTI_Launch
  (params (CamRot :type Rotator) (P0 :type Vector) (P2 :type Vector) (Apex :type Vector) (StartTime :type Float%20%28double-precision%29))
  (Variables|Default|SetP0 P0)
  (Variables|Default|SetP2 P2)
  (Variables|Default|SetApex Apex)
  (bind _output_get (Variables|Default|SetP1 (- (* (Math|Vector|MakeVector (.X (Math|Vector|BreakVector (* (+ (Variables|Default|GetP0) (Variables|Default|GetP2)) 0.5))) (.Y (Math|Vector|BreakVector (* (+ (Variables|Default|GetP0) (Variables|Default|GetP2)) 0.5))) (.z (Variables|Default|GetApex))) 2.0) (* (+ (Variables|Default|GetP0) (Variables|Default|GetP2)) 0.5))))
  (Game|SpawnActorfromClass "/Game/Weapons/Hook/Grapple/BP_GrappleProjectile.BP_GrappleProjectile_C" (Math|Transform|MakeTransform (Variables|Default|GetP0) CamRot "1.000000,1.000000,1.000000") "Undefined" "MultiplyWithRoot" 0 (Variables|Default|GetP0) (Variables|Default|GetP1) (Variables|Default|GetP2) StartTime (/ (+ (Math|Vector|Distance(Vector) (Variables|Default|GetP0) (Variables|Default|GetP1)) (Math|Vector|Distance(Vector) (Variables|Default|GetP1) (Variables|Default|GetP2))) (Variables|Default|GetProjectileSpeed)) (Variables|Default|GetHero)))

(event Custom|SERV_Launch
  (params (CamLoc :type Vector) (CamRot :type Rotator) (Hero :type Character%20Object%20Reference))
  (bind (_p2 _apex) (CallFunction|TraceforSurface CamLoc CamRot Hero 1e+04 4.0 1e+02))
  (CallFunction|MULTILaunch CamRot CamLoc _p2 _apex (GameState|GetServerWorldTimeSeconds (Game|GetGameState))))

(event Input|EnhancedActionEvents|EnhancedInputActionIA_Hook_Launch
  (params (ActionValue :type Boolean) (ElapsedSeconds :type Float%20%28double-precision%29) (TriggeredSeconds :type Float%20%28double-precision%29) (InputAction :type Input%20Action%20Object%20Reference :default "/Game/Input/Actions/IA_Hook_Launch.IA_Hook_Launch"))
  (bind _herocam (Variables|Default|GetHeroCam))
  (bind _returnvalue (Transformation|GetWorldTransform _herocam))
  (:Started
    (Networking|SwitchHasAuthority
      (:Authority
        (bind (_p2 _apex) (CallFunction|TraceforSurface (.location _returnvalue) (.rotation _returnvalue) 0 1e+04 4.0 1e+02))
        (CallFunction|MULTILaunch (.rotation _returnvalue) (.location _returnvalue) _p2 _apex (GameState|GetServerWorldTimeSeconds (Game|GetGameState))))
      (:Remote
        (CallFunction|SERVLaunch (.location _returnvalue) (.rotation _returnvalue) (Variables|Default|GetHero))))))

(event EventBeginPlay
  (Utilities|FlowControl|Sequence
    (:then_0
      (bind _ascharacter (Utilities|Casting|CastToCharacter (Components|GetOwner)))
      (Variables|Default|SetHero _ascharacter)
      (bind _returnvalue (Game|SpawnActorfromClass "/Game/Weapons/Hook/Grapple/BP_GrappleArm.BP_GrappleArm_C" (Math|Transform|MakeTransform "0, 0, 0" "0, 0, 0" "1.000000,1.000000,1.000000") "Undefined" "MultiplyWithRoot" 0 0))
      (bind _output_get (Variables|Default|SetHookArm _returnvalue))
      (Transformation|AttachComponentToComponent _output_get (Variables|/Script/Engine.Character|GetMesh (Variables|Default|GetHero)) "HandGrip_L" "SnapToTarget" "SnapToTarget" "KeepWorld" true))
    (:then_1
      (Variables|Default|SetHeroCam (Actor|GetComponentbyClass (Variables|Default|GetHero) "/Script/Engine.CameraComponent")))))

(fn TraceforSurface
  (params (CamLoc :type Vector) (CamRot :type Rotator) (Hero :type Character%20Object%20Reference) (DefaultTraceDistance :type Float%20%28double-precision%29) (TrajectoryDistance :type Float%20%28double-precision%29) (Debug_ProjectileRadius :type Float%20%28double-precision%29))
  (LocalVariables|SetFinalTracePoint (+ CamLoc (* (Math|Vector|GetForwardVector CamRot) DefaultTraceDistance)))
  (bind (_outhit _returnvalue) (Collision|LineTraceByChannel CamLoc (LocalVariables|GetFinalTracePoint) "TraceTypeQuery1" false (Utilities|Array|MakeArray Hero) "None"))
  (bind _tossvelocity (Class|GameplayStatics|BlueprintSuggestProjectileVelocity CamLoc (Math|Vector|SelectVector (.ImpactPoint (Collision|BreakHitResult _outhit)) (LocalVariables|GetFinalTracePoint) _returnvalue) (Variables|Default|GetProjectileSpeed) 0.0 "DoNotTrace" Debug_ProjectileRadius false false false))
  (bind (_outhit_2 _outpathpositions _outlasttracedestination) (Class|GameplayStatics|BlueprintPredictProjectilePathbyObjectType CamLoc _tossvelocity false Debug_ProjectileRadius (Utilities|Array|MakeArray "ObjectTypeQuery11") false (Utilities|Array|MakeArray Hero) "None" 1e+01 (* (/ 1.0 TrajectoryDistance) 2.0) TrajectoryDistance))
  (return _outlasttracedestination (Utilities|Array|Get(acopy) _outpathpositions 1)))