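; Grappling hook projectile that flies out from the grapple arm, sticks to what it hits and can be recalled.
; Tick moves it along a curve-eased quadratic Bézier using server world time, line-tracing between steps to attach at impact with adjustable penetration.
; Without a hit, the server starts recall near flight end.
; Recall detaches and lerps it back to its owner, where the server resets BP_GrappleArm and destroys it.
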(event Custom|StartRecalling
  (Transformation|DetachFromActor "KeepRelative" "KeepRelative" "KeepRelative")
  (Variables|Recall|SetRecallStartTime (GameState|GetServerWorldTimeSeconds (Game|GetGameState)))
  (Variables|Recall|SetRecallStartPos (Transformation|GetActorLocation))
  (Variables|Recall|SetIsRecalling? true))

(event EventTick
  (params (DeltaSeconds :type Float%20%28single-precision%29))
  (bind _returnvalue (Game|GetGameState))
  (bind _returnvalue_2 (Game|GetGameState))
  (bind _launchstarttime (Variables|Launch|GetLaunchStartTime))
  (bind _launchduration (Variables|Launch|GetLaunchDuration))
  (bind _recallstarttime (Variables|Recall|GetRecallStartTime))
  (bind _recallduration (Variables|Recall|GetRecallDuration))
  (bind _returnvalue_3 (GameState|GetServerWorldTimeSeconds _returnvalue))
  (bind _returnvalue_4 (GameState|GetServerWorldTimeSeconds _returnvalue_2))
  (bind _returnvalue_5 (- _returnvalue_4 _recallstarttime))
  (bind _returnvalue_6 (- _returnvalue_3 _launchstarttime))
  (bind _returnvalue_7 (/ _returnvalue_6 _launchduration))
  (bind _returnvalue_8 (/ _returnvalue_5 _recallduration))
  (bind _returnvalue_9 (Math|Float|Clamp(Float) _returnvalue_8 0.0))
  (bind _returnvalue_10 (Math|Float|Clamp(Float) _returnvalue_7 0.005))
  (if (Variables|Recall|GetIsRecalling?)
    (Transformation|SetActorLocation (Math|Vector|Lerp(Vector) (Variables|Recall|GetRecallStartPos) (Transformation|GetActorLocation (Components|GetOwner)) (Math|Curves|GetFloatValue (Variables|Launch|GetCurve) _returnvalue_9)) false false)
    (if (>= _returnvalue_9 1.0)
      (Networking|SwitchHasAuthority
        (:Authority
          (Utilities|FlowControl|Sequence
            (:then_0
              (bind _asbp_grapple_arm (Utilities|Casting|CastToBP_GrappleArm (Components|GetOwner)))
              (Variables|/Game/Weapons/Hook/Grapple/BP_GrappleArm.BP_GrappleArm_C|SetHookFired? _asbp_grapple_arm false)
              (Variables|/Game/Weapons/Hook/Grapple/BP_GrappleArm.BP_GrappleArm_C|SetProjectile _asbp_grapple_arm 0)
              (Default|UpdateHookVisuals _asbp_grapple_arm))
            (:then_1
              (Actor|DestroyActor))))))
    (elif (> (Variables|Launch|GetLaunchStartTime) 0.0)
      (if (Math|Float|NearlyEqual(Float) _returnvalue_10 1.0 0.05) ; Has reached destinaion ?
        (Networking|SwitchHasAuthority
          (:Authority
            (Utilities|FlowControl|DoOnce false
              (:Completed
                (if (not (Variables|Recall|GetIsRecalling?))
                  (CallFunction|StartRecalling))))))
        (else
          (bind _bezpos (CallFunction|GetBezierPos (Variables|Launch|GetP0) (Variables|Launch|GetP1) (Variables|Launch|GetP2) (Math|Curves|GetFloatValue (Variables|Launch|GetCurve) _returnvalue_10)))
          (Transformation|SetActorLocation _bezpos false false)
          (bind _output_get (Variables|Launch|SetBez%20Pos_Prev (Variables|Launch|GetBez%20Pos)))
          (bind (_outhit _returnvalue_11) (Collision|LineTraceForObjects _output_get _bezpos (Utilities|Array|MakeArray "ObjectTypeQuery1" "ObjectTypeQuery8") false (Utilities|Array|MakeArray (Components|GetOwner) (Variables|Actor|GetInstigator)) "None"))
          (Variables|Launch|SetBez%20Pos _bezpos)
          (if _returnvalue_11
            (Utilities|FlowControl|Sequence
              (:then_0
                (Actor|Tick|SetActorTickEnabled false))
              (:then_1
                (Transformation|SetActorLocation (+ (.ImpactPoint (Collision|BreakHitResult _outhit)) (* (Math|Vector|GetUnitDirection(Vector) (Variables|Launch|GetBez%20Pos) (Variables|Launch|GetBez%20Pos_Prev)) (* (.sphereradius (StaticMesh|GetBounds (Variables|/Script/Engine.StaticMeshComponent|GetStaticMesh (Variables|Default|GetHook)))) 2.0 (Math|Float|Clamp(Float) (- 1.0 (/ (Variables|ProjectileParams|GetSurfacePenetration) 1e+02)) 0.01)))) false false)
                (Transformation|AttachComponentToComponent (.HitComponent (Collision|BreakHitResult _outhit)) "None" "KeepWorld" "KeepWorld" "KeepWorld" true)
                (Transformation|SetAbsolute (Variables|Default|GetHook) false false true)
                (Transformation|SetActorScale3D "1.000000,1.000000,1.000000")))))))))

(fn ConstructionScript)

(fn GetBezierPos
  (params (P0 :type Vector) (P1 :type Vector) (P2 :type Vector) (t :type Float%20%28double-precision%29))
  (return (Math|Vector|Lerp(Vector) (Math|Vector|Lerp(Vector) P0 P1 t) (Math|Vector|Lerp(Vector) P1 P2 t) t)))

(fn OnRepIsRecalling?
  (Transformation|DetachFromActor "KeepRelative" "KeepRelative" "KeepRelative"))