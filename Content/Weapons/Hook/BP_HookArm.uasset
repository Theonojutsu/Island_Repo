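; BP_HookArm is a hook arm pickup that equips itself to the first eligible Character overlapping its PhysHook sphere.
; It skips Characters that already have a BP_HookArm attached, and a DoOnce keeps it from being claimed again.
; On pickup it adds an AC_Hook component to the Character, switches PhysHook to a PhysicsBody, resizes the sphere, and snaps to the left-hand grip socket.
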(event OnComponentBeginOverlap(PhysHook)
  (params (OverlappedComponent :type Primitive%20Component%20Object%20Reference) (OtherActor :type Actor%20Object%20Reference) (OtherComp :type Primitive%20Component%20Object%20Reference) (OtherBodyIndex :type Integer) (bFromSweep :type Boolean) (SweepResult :type Hit%20Result%20Structure%20%28by%20ref%29))
  (bind _ascharacter (Utilities|Casting|CastToCharacter OtherActor))
  (Variables|Default|SetHasAlreadyHook false)
  (bind _array_element (Utilities|Array|ForEachLoopwithBreak (Actor|GetAttachedActors _ascharacter true false) :!label _label)
    (:LoopBody
      (Class|KismetSystemLibrary|IsObjectOfSoftClass _array_element "/Game/Weapons/Hook/BP_HookArm.BP_HookArm_C"
        (:True
          (Variables|Default|SetHasAlreadyHook true)
          (goto _label Break))))
    (:Completed
      (if (not (Variables|Default|GetHasAlreadyHook))
        (Utilities|FlowControl|DoOnce false
          (:Completed
            (Game|AddComponentbyClass _ascharacter "/Game/Weapons/Hook/AC_Hook.AC_Hook_C" _ascharacter self)
            (CallFunction|AttachSelftoHero _ascharacter)))))))

(event Custom|AttachSelfToHero
  (params (Character :type Character%20Object%20Reference))
  (Utilities|FlowControl|Sequence
    (:then_0
      (Collision|SetCollisionObjectType (Variables|Default|GetPhysHook) "ECC_PhysicsBody")
      (Components|Sphere|SetSphereRadius (Variables|Default|GetPhysHook) 18.0 true))
    (:then_1
      (Transformation|AttachComponentToComponent self (Variables|/Script/Engine.Character|GetMesh Character) "HandGrip_L" "SnapToTarget" "SnapToTarget" "KeepWorld" true))))

(fn ConstructionScript)