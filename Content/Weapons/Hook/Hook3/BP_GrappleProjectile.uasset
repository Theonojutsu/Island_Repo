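; BP_GrappleProjectile is a grapple hook projectile that moves along a curved path over a set duration.
; Once StartTime is set, Tick derives normalized progress from server world time, so position follows a shared clock rather than accumulated deltas.
; A float curve reshapes that progress, which GetBezierPos turns into a quadratic Bezier position through P0, P1 and P2.
; An ApexBias time remap is present but unused.
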(event EventTick
  (params (DeltaSeconds :type Float%20%28single-precision%29))
  (if (> (Variables|Default|GetStartTime) 0.0)
    (bind _bezpos (CallFunction|GetBezierPos (Variables|Default|GetP0) (Variables|Default|GetP1) (Variables|Default|GetP2) (Math|Curves|GetFloatValue (Variables|Default|GetCurve) (Math|Float|Clamp(Float) (/ (- (GameState|GetServerWorldTimeSeconds (Game|GetGameState)) (Variables|Default|GetStartTime)) (Variables|Default|GetDuration))))))
    (Transformation|SetActorLocation _bezpos false false)))

(fn ConstructionScript)

(fn GetBezierPos
  (params (P0 :type Vector) (P1 :type Vector) (P2 :type Vector) (t :type Float%20%28double-precision%29))
  (return (Math|Vector|Lerp(Vector) (Math|Vector|Lerp(Vector) P0 P1 t) (Math|Vector|Lerp(Vector) P1 P2 t) t)))