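; Grappling hook component for a Character: attaches an arm to the left hand and fires BP_GrappleProjectile on input.
; The server line-traces from the camera, then uses a suggested toss velocity and coarse path prediction to find an apex sample and end point.
; A multicast derives a quadratic Bezier control point and spawns each machine's projectile with server start time and length-based duration.
; Debug drawing of the path and points is enabled.
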(event Custom|MULTI_Launch
  (params (CamRot :type Rotator) (P0 :type Vector) (Apex :type Vector) (P2 :type Vector) (StartTime :type Float%20%28double-precision%29))
  (Variables|Default|SetP0 P0)
  (Variables|Default|SetP2 P2)
  (Variables|Default|SetApex Apex)
  (bind _output_get (Variables|Default|SetP1 (- (* (Math|Vector|MakeVector (.X (Math|Vector|BreakVector (* (+ (Variables|Default|GetP0) (Variables|Default|GetP2)) 0.5))) (.Y (Math|Vector|BreakVector (* (+ (Variables|Default|GetP0) (Variables|Default|GetP2)) 0.5))) (.z (Variables|Default|GetApex))) 2.0) (* (+ (Variables|Default|GetP0) (Variables|Default|GetP2)) 0.5))))
  (Rendering|Debug|DrawDebugBox _output_get "500.000000,500.000000,500.000000" "(R=0.000000,G=0.123698,B=1.000000,A=1.000000)" "0, 0, 0" 9999.0 1e+01)
  (Rendering|Debug|DrawDebugBox (Variables|Default|GetApex) "500.000000,500.000000,500.000000" "(R=1.000000,G=0.084888,B=0.000000,A=1.000000)" "0, 0, 0" 9999.0 1e+01)
  (Game|SpawnActorfromClass "/Game/Weapons/Hook/Hook3/BP_GrappleProjectile.BP_GrappleProjectile_C" (Math|Transform|MakeTransform (Variables|Default|GetP0) CamRot "1.000000,1.000000,1.000000") "Undefined" "MultiplyWithRoot" 0 (Variables|Default|GetP0) (Variables|Default|GetP1) (Variables|Default|GetP2) StartTime (/ (+ (Math|Vector|Distance(Vector) (Variables|Default|GetP0) (Variables|Default|GetP1)) (Math|Vector|Distance(Vector) (Variables|Default|GetP1) (Variables|Default|GetP2))) (Variables|Default|GetSpeed)) 0.0 0))

(event Custom|SERV_Launch
  (params (CamLoc :type Vector) (CamRot :type Rotator) (P0 :type Vector))
  (bind (_camrot_out _p0_out _p2_out _starttime _apex) (CallFunction|TracewithParams CamLoc CamRot P0))
  (CallFunction|MULTILaunch _camrot_out _p0_out _apex _p2_out _starttime))

(event Input|EnhancedActionEvents|EnhancedInputActionIA_Hook_Launch
  (params (ActionValue :type Boolean) (ElapsedSeconds :type Float%20%28double-precision%29) (TriggeredSeconds :type Float%20%28double-precision%29) (InputAction :type Input%20Action%20Object%20Reference :default "/Game/Input/Actions/IA_Hook_Launch.IA_Hook_Launch"))
  (bind _herocam (Variables|Default|GetHeroCam))
  (bind _returnvalue (Transformation|GetWorldRotation _herocam))
  (bind _returnvalue_2 (Transformation|GetWorldLocation _herocam))
  (:Started
    (Networking|SwitchHasAuthority
      (:Authority
        (bind (_camrot_out _p0_out _p2_out _starttime _apex) (CallFunction|TracewithParams _returnvalue_2 _returnvalue _returnvalue_2))
        (CallFunction|MULTILaunch _camrot_out _p0_out _apex _p2_out _starttime))
      (:Remote
        (CallFunction|SERVLaunch _returnvalue_2 _returnvalue _returnvalue_2)))))

(event EventBeginPlay
  (Utilities|FlowControl|Sequence
    (:then_0
      (bind _ascharacter (Utilities|Casting|CastToCharacter (Components|GetOwner)))
      (Variables|Default|SetHero _ascharacter)
      (bind _returnvalue (Game|SpawnActorfromClass "/Game/Weapons/Hook/Hook3/BP_GrappleArm.BP_GrappleArm_C" (Math|Transform|MakeTransform "0, 0, 0" "0, 0, 0" "1.000000,1.000000,1.000000") "Undefined" "MultiplyWithRoot" 0 0))
      (bind _output_get (Variables|Default|SetHookArm _returnvalue))
      (Transformation|AttachComponentToComponent _output_get (Variables|/Script/Engine.Character|GetMesh (Variables|Default|GetHero)) "HandGrip_L" "SnapToTarget" "SnapToTarget" "KeepWorld" true))
    (:then_1
      (Variables|Default|SetHeroCam (Actor|GetComponentbyClass (Variables|Default|GetHero) "/Script/Engine.CameraComponent")))))

(fn TraceforSurface
  (params (CamLoc :type Vector) (CamRot :type Rotator) (Hero :type Character%20Object%20Reference))
  (bind _returnvalue (Math|Float|MakeLiteralFloat 4.0))
  (bind _returnvalue_2 (Math|Vector|GetForwardVector CamRot))
  (bind _returnvalue_3 (Math|Float|MakeLiteralFloat 1e+04))
  (bind _returnvalue_4 (* _returnvalue_2 _returnvalue_3))
  (bind _returnvalue_5 (+ CamLoc _returnvalue_4))
  (bind (_outhit _returnvalue_6) (Collision|LineTraceByChannel CamLoc _returnvalue_5 "TraceTypeQuery1" false (Utilities|Array|MakeArray Hero) "None"))
  (bind _tossvelocity (Class|GameplayStatics|BlueprintSuggestProjectileVelocity CamLoc (Math|Vector|SelectVector (.ImpactPoint (Collision|BreakHitResult _outhit)) _returnvalue_5 _returnvalue_6) (Variables|Default|GetSpeed) 0.0 "DoNotTrace" (Variables|Default|GetProjectileRadius) false false false))
  (bind (_outhit_2 _outpathpositions _outlasttracedestination) (Class|GameplayStatics|BlueprintPredictProjectilePathbyObjectType CamLoc _tossvelocity true 5e+02 (Utilities|Array|MakeArray "ObjectTypeQuery5") false (Utilities|Array|MakeArray Hero) "ForDuration" 1e+01 (* (/ 1.0 _returnvalue) 2.0) _returnvalue))
  (return _outlasttracedestination (Utilities|Array|Get(acopy) _outpathpositions 1)))

(fn TracewithParams
  (params (CamLoc :type Vector) (CamRot :type Rotator) (P0 :type Vector))
  (bind (_p2 _apex) (CallFunction|TraceforSurface CamLoc CamRot (Variables|Default|GetHero)))
  (return CamRot P0 _p2 (GameState|GetServerWorldTimeSeconds (Game|GetGameState)) _apex))