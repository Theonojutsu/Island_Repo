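; Grappling hook component for a Character that fires, pulls toward and recalls a hook projectile with a cable from the left hand.
; On impact the projectile sticks to the hit component, and its physical surface type becomes the state that routes later inputs.
; Holding left click applies force toward the hook in Flying mode with slight side steering and widened FOV.
; Releasing it restores Falling and, like right click, triggers a timeline-driven recall.
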(event Custom|UpdateFOV
  (params (Increase? :type Boolean))
  (if Increase?
    (bind _alpha (Utilities|ComponentTimeline 4.0 "/Game/Libraries/Data/Curves/C_Linear.C_Linear" :!label _label)
      (:Update
        (Camera|SetFieldOfView (Variables|Default|GetHero_Cam) (Math|Float|Lerp 9e+01 1.1e+02 _alpha))))
    (else
      (goto _label Reverse))))

(event Custom|HookSticked
  (params (HitComponent :type Primitive%20Component%20Object%20Reference) (OtherActor :type Actor%20Object%20Reference) (OtherComp :type Primitive%20Component%20Object%20Reference) (NormalImpulse :type Vector) (Hit :type Hit%20Result%20Structure%20%28by%20ref%29))
  (if (!= (Components|GetOwner OtherComp) (Components|GetOwner))
    (Utilities|FlowControl|Sequence
      (:then_0
        (Components|Activation|SetActive (Variables|/Game/Weapons/Hook/Hook2/BP_ProjectileHook.BP_ProjectileHook_C|GetProjectileMovement (Variables|Default|GetProjectileHook)) false false))
      (:then_1
        (Transformation|AttachComponentToComponent (Variables|Default|GetProjectileHook) OtherComp "None" "KeepWorld" "KeepWorld" "KeepWorld" true)
        (Transformation|SetAbsolute (Variables|/Script/Engine.Actor|GetRootComponent (Variables|Default|GetProjectileHook)) false false true)
        (Transformation|SetActorScale3D (Variables|Default|GetProjectileHook) "1.000000,1.000000,1.000000"))
      (:then_2
        (Camera|PlayWorldCameraShake "/Game/FirstPerson/Camera/CS_ShakeToSurface.CS_ShakeToSurface_C" (Transformation|GetActorLocation (Variables|Default|GetHero)) 0.0 5e+02))
      (:then_3
        (Variables|Default|SetSurface%20Type (Variables|/Script/PhysicsCore.PhysicalMaterial|GetSurfaceType (.PhysMat (Collision|BreakHitResult Hit))))))))

(event Input|EnhancedActionEvents|EnhancedInputActionIA_Move
  (params (ActionValue :type Vector%202D%20Structure) (ElapsedSeconds :type Float%20%28double-precision%29) (TriggeredSeconds :type Float%20%28double-precision%29) (InputAction :type Input%20Action%20Object%20Reference :default "/Game/Input/Actions/IA_Move.IA_Move"))
  (Variables|Default|SetAxis_Move (Math|Vector2D|MakeVector2D (.x ActionValue) (.y ActionValue))))

(event Input|EnhancedActionEvents|EnhancedInputActionIA_E
  (params (ActionValue :type Boolean) (ElapsedSeconds :type Float%20%28double-precision%29) (TriggeredSeconds :type Float%20%28double-precision%29) (InputAction :type Input%20Action%20Object%20Reference :default "/Game/Input/Actions/IA_E.IA_E"))
  (bind _hero (Variables|Default|GetHero))
  (bind _hero_cam (Variables|Default|GetHero_Cam))
  (:Started
    (switch Utilities|FlowControl|Switch|SwitchonEPhysicalSurface (Variables|Default|GetSurface%20Type)
      (:SurfaceType3
        _)
      (:SurfaceType4
        _))
    (Utilities|FlowControl|Sequence
      (:then_0
        (Development|SetHiddeninGame (Variables|/Game/Weapons/Hook/Hook2/BP_HookBase.BP_HookBase_C|GetHookPiece (Variables|Default|GetHookBase)) true false)
        (Development|SetHiddeninGame (Variables|Default|GetCable) false false)
        (Variables|Default|SetSurface%20Type "SurfaceType4"))
      (:then_1
        (bind _returnvalue (Game|SpawnActorfromClass "/Game/Weapons/Hook/Hook2/BP_ProjectileHook.BP_ProjectileHook_C" (Math|Transform|MakeTransform (+ (* (Math|Vector|GetRightVector _hero_cam) -10) (* (Math|Vector|GetForwardVector _hero_cam) 25) (* (Math|Vector|GetUpVector _hero_cam) -25) (Transformation|GetWorldLocation _hero_cam)) (Math|Rotator|MakeRotfromX (Math|Vector|GetForwardVector _hero_cam)) "1.000000,1.000000,1.000000") "AlwaysSpawn" "MultiplyWithRoot" _hero _hero))
        (bind _output_get (Variables|Default|SetProjectileHook _returnvalue))
        (Class|CableComponent|SetAttachEndtoComponent (Variables|Default|GetCable) (Variables|/Game/Weapons/Hook/Hook2/BP_ProjectileHook.BP_ProjectileHook_C|GetHook _output_get) "CableAttachment"))
      (:then_2
        (Collision|BindEventtoOnComponentHit (Variables|/Game/Weapons/Hook/Hook2/BP_ProjectileHook.BP_ProjectileHook_C|GetHook (Variables|Default|GetProjectileHook)) (delegate Custom|HookSticked))))))

(event Input|EnhancedActionEvents|EnhancedInputActionIA_RightClick
  (params (ActionValue :type Boolean) (ElapsedSeconds :type Float%20%28double-precision%29) (TriggeredSeconds :type Float%20%28double-precision%29) (InputAction :type Input%20Action%20Object%20Reference :default "/Game/Input/Actions/IA_RightClick.IA_RightClick"))
  (:Started
    (switch Utilities|FlowControl|Switch|SwitchonEPhysicalSurface (Variables|Default|GetSurface%20Type)
      (:SurfaceType_Default
        _)
      (:SurfaceType1
        _)
      (:SurfaceType2
        _))
    (Utilities|FlowControl|DoOnce false
      (:Completed
        (Camera|PlayWorldCameraShake "/Game/FirstPerson/Camera/CS_ShakeToSurface.CS_ShakeToSurface_C" (Transformation|GetActorLocation (Variables|Default|GetHero)) 0.0 5e+02)
        (Variables|Default|SetRecall_HookLocation (Transformation|GetActorLocation (Variables|Default|GetProjectileHook)))
        (bind _alpha (Utilities|ComponentTimeline 2.0 "/Game/Libraries/Data/Curves/C_Rise.C_Rise") ; enters at PlayFromStart
          (:Update
            (Transformation|SetActorLocation (Variables|Default|GetProjectileHook) (Math|Vector|Lerp(Vector) (Variables|Default|GetRecall_HookLocation) (Transformation|GetActorLocation (Variables|Default|GetHookBase)) _alpha) false false))
          (:Completed
            (bind _projectilehook (Variables|Default|GetProjectileHook)
              (:then
                (Actor|DestroyActor _projectilehook)
                (Development|SetHiddeninGame (Variables|/Game/Weapons/Hook/Hook2/BP_HookBase.BP_HookBase_C|GetHookPiece (Variables|Default|GetHookBase)) false false)
                (Development|SetHiddeninGame (Variables|Default|GetCable) true false)
                (Variables|Default|SetSurface%20Type "SurfaceType4"))
              (:else))))))))

(event Input|EnhancedActionEvents|EnhancedInputActionIA_LeftClick
  (params (ActionValue :type Boolean) (ElapsedSeconds :type Float%20%28double-precision%29) (TriggeredSeconds :type Float%20%28double-precision%29) (InputAction :type Input%20Action%20Object%20Reference :default "/Game/Input/Actions/IA_LeftClick.IA_LeftClick"))
  (bind _returnvalue (Components|GetOwner))
  (bind _hero (Variables|Default|GetHero))
  (bind _charactermovement (Variables|/Script/Engine.Character|GetCharacterMovement _hero))
  (:Triggered
    (switch Utilities|FlowControl|Switch|SwitchonEPhysicalSurface (Variables|Default|GetSurface%20Type)
      (:SurfaceType_Default
        _)
      (:SurfaceType2
        _))
    (if (Class|NavMovementInterface|IsFlying _charactermovement)
      _
      (else
        (Pawn|Components|CharacterMovement|SetMovementMode _charactermovement "MOVE_Flying" 0)))
    (Physics|AddForce (Variables|/Script/Engine.Character|GetCharacterMovement (Variables|Default|GetHero)) (* (Math|Vector|Normalize (+ (Math|Vector|GetUnitDirection(Vector) (Transformation|GetActorLocation _returnvalue) (Transformation|GetActorLocation (Variables|Default|GetProjectileHook))) (* (* (Transformation|GetActorRightVector _returnvalue) (.x (Variables|Default|GetAxis_Move))) 0.15))) 2.5e+05)))
  (:Started
    (switch Utilities|FlowControl|Switch|SwitchonEPhysicalSurface (Variables|Default|GetSurface%20Type)
      (:SurfaceType_Default
        _)
      (:SurfaceType2
        _))
    (CallFunction|UpdateFOV true))
  (:Canceled
    (switch Utilities|FlowControl|Switch|SwitchonEPhysicalSurface (Variables|Default|GetSurface%20Type) :!label _label
      (:SurfaceType_Default
        _)
      (:SurfaceType1
        _)
      (:SurfaceType2
        _))
    (CallFunction|UpdateFOV false)
    (Pawn|Components|CharacterMovement|SetMovementMode (Variables|/Script/Engine.Character|GetCharacterMovement (Variables|Default|GetHero)) "MOVE_Falling" 0)
    (Utilities|FlowControl|DoOnce false
      (:Completed
        (Camera|PlayWorldCameraShake "/Game/FirstPerson/Camera/CS_ShakeToSurface.CS_ShakeToSurface_C" (Transformation|GetActorLocation (Variables|Default|GetHero)) 0.0 5e+02)
        (Variables|Default|SetRecall_HookLocation (Transformation|GetActorLocation (Variables|Default|GetProjectileHook)))
        (bind _alpha (Utilities|ComponentTimeline 2.0 "/Game/Libraries/Data/Curves/C_Rise.C_Rise") ; enters at PlayFromStart
          (:Update
            (Transformation|SetActorLocation (Variables|Default|GetProjectileHook) (Math|Vector|Lerp(Vector) (Variables|Default|GetRecall_HookLocation) (Transformation|GetActorLocation (Variables|Default|GetHookBase)) _alpha) false false))
          (:Completed
            (bind _projectilehook (Variables|Default|GetProjectileHook)
              (:then
                (Actor|DestroyActor _projectilehook)
                (Development|SetHiddeninGame (Variables|/Game/Weapons/Hook/Hook2/BP_HookBase.BP_HookBase_C|GetHookPiece (Variables|Default|GetHookBase)) false false)
                (Development|SetHiddeninGame (Variables|Default|GetCable) true false)
                (Variables|Default|SetSurface%20Type "SurfaceType4"))
              (:else)))))))
  (:Completed
    (goto _label)))

(event EventBeginPlay
  (Utilities|FlowControl|Sequence
    (:then_0
      (bind _ascharacter (Utilities|Casting|CastToCharacter (Components|GetOwner)))
      (Variables|Default|SetHero _ascharacter))
    (:then_1
      (Utilities|IsValid (Actor|GetComponentbyClass (Variables|Default|GetHero) "/Script/Engine.CameraComponent")
        (:Is%20Valid
          (Variables|Default|SetHero_Cam (Actor|GetComponentbyClass (Variables|Default|GetHero) "/Script/Engine.CameraComponent")))))
    (:then_2
      (bind _returnvalue (Game|SpawnActorfromClass "/Game/Weapons/Hook/Hook2/BP_HookBase.BP_HookBase_C" (Math|Transform|MakeTransform "0, 0, 0" "0, 0, 0" "1.000000,1.000000,1.000000") "Undefined" "MultiplyWithRoot" (Variables|Default|GetHero) (Variables|Default|GetHero)))
      (bind _output_get (Variables|Default|SetHookBase _returnvalue))
      (Variables|Default|SetCable (Variables|/Game/Weapons/Hook/Hook2/BP_HookBase.BP_HookBase_C|GetCable _output_get))
      (Transformation|AttachComponentToComponent _output_get (Variables|/Script/Engine.Character|GetMesh (Variables|Default|GetHero)) "HandGrip_L" "SnapToTarget" "SnapToTarget" "KeepWorld" true))))

(fn NewFunction
  (bind (_outhit _outpathpositions _outlasttracedestination) (Class|GameplayStatics|BlueprintPredictProjectilePathbyObjectType "0, 0, 0" "0, 0, 0" true 0.0 (Utilities|Array|MakeArray "ObjectTypeQuery5") false 0 "ForDuration" 2e+01))
  (for _array_element _outpathpositions
    (if (>= (.Z (Math|Vector|BreakVector _array_element)) -999999999.0)
      (LocalVariables|SetNewLocalVar_0 (.Z (Math|Vector|BreakVector _array_element)))
      (LocalVariables|SetNewLocalVar _array_element)))
  (return (LocalVariables|GetNewLocalVar) _outlasttracedestination "0, 0, 0"))