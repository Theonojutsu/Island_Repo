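; Grappling hook actor that attaches to the first Character hitting it, then lets that player fire and pull toward a physics hook.
; E launches the hook along a camera trace, and hits stick based on physical surface type.
; Holding left click flies the character toward it with mouse-driven sideways steering.
; A looping timer recalls the hook by force after timeout, right click or left-click release, reattaching it when close.
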(event OnComponentHit(PhysHook)
  (params (HitComponent :type Primitive%20Component%20Object%20Reference) (OtherActor :type Actor%20Object%20Reference) (OtherComp :type Primitive%20Component%20Object%20Reference) (NormalImpulse :type Vector :default "0, 0, 0") (Hit :type Hit%20Result%20Structure%20%28by%20ref%29))
  (bind (_bblockinghit _binitialoverlap _time _distance _location _impactpoint _normal _impactnormal _physmat) (Collision|BreakHitResult Hit))
  (Variables|Default|GetHero
    (:then
      ;[0.15 0.15 0.15 0.5 50] Stick to surface
      (if (!= OtherActor (Variables|Default|GetHero))
        (Utilities|FlowControl|DoOnce false
          (:Completed
            (bind _output_get (Variables|Default|SetSurface%20Type (Variables|/Script/PhysicsCore.PhysicalMaterial|GetSurfaceType _physmat)))
            (if (and (Utilities|Enum|NotEqual(Enum) _output_get "SurfaceType4") (Utilities|Enum|NotEqual(Enum) _output_get "SurfaceType3"))
              (Transformation|SetWorldLocation (Variables|Default|GetPhysHook) _impactpoint false true)
              (Physics|SetSimulatePhysics (Variables|Default|GetPhysHook) false)
              (Utilities|Time|ClearandInvalidateTimerbyHandle (Variables|Default|GetLaunchHookTimer))
              (Camera|PlayWorldCameraShake "/Game/FirstPerson/Camera/CS_ShakeToSurface.CS_ShakeToSurface_C" (Transformation|GetActorLocation (Variables|Default|GetHero)) 0.0 5e+02)
              (CallFunction|ToggleHookCollision false))))))
    (:else
      ;[0.15 0.15 0.15 0.5 50] Attach to Player
      (bind _ascharacter (Utilities|Casting|CastToCharacter OtherActor))
      (Utilities|FlowControl|DoOnce false
        (:Completed
          (Utilities|FlowControl|Sequence
            (:then_0
              (Variables|Default|SetHero _ascharacter)
              (Transformation|AttachComponentToComponent self (Variables|/Script/Engine.Character|GetMesh _ascharacter) "HandGrip_L" "SnapToTarget" "SnapToTarget" "KeepWorld" true))
            (:then_1
              (Collision|IgnoreActorwhenMoving (Variables|/Script/Engine.Character|GetCapsuleComponent _ascharacter) self true))
            (:then_2
              (Variables|Default|SetHeroCam (Actor|GetComponentbyClass (Variables|Default|GetHero) "/Script/Engine.CameraComponent")))))))))

(event Custom|ResetHookDetection
  ;[0.15 0.15 0.15 0.5 50] Stick to surface
  (Utilities|FlowControl|DoOnce false) ; enters at Reset
)

(event Custom|CheckSurface
  (bind _physhook (Variables|Default|GetPhysHook))
  (bind _hookbase (Variables|Default|GetHookBase))
  (bind _physhook_2 (Variables|Default|GetPhysHook))
  (bind _hookbase_2 (Variables|Default|GetHookBase))
  (bind _physhook_3 (Variables|Default|GetPhysHook))
  (bind _returnvalue (Transformation|GetWorldLocation _physhook))
  (bind _returnvalue_2 (Transformation|GetWorldLocation _hookbase))
  (bind _returnvalue_3 (Transformation|GetWorldLocation _hookbase_2))
  (bind _returnvalue_4 (Transformation|GetWorldLocation _physhook_2))
  (bind _returnvalue_5 (Math|Vector|Distance(Vector) _returnvalue _returnvalue_2))
  ;[0.15 0.15 0.15 0.5 50] Check for Hook exceeding max travel time
  (bind _output_get (Variables|Default|SetHookRevoveryDelay (+ (Utilities|Time|GetWorldDeltaSeconds) (stale _output_get))))
  (if (> _output_get 1.0) ; Hook's max travel time reached ?
    ;[0.15 0.15 0.15 0.5 50] Recall Hook
    (Utilities|FlowControl|Sequence
      (:then_0
        (Utilities|FlowControl|DoOnce false :!label _label
          (:Completed
            (CallFunction|ToggleHookCollision false))))
      (:then_1
        (Class|PrimitiveComponent|SetPhysicsAngularVelocityinDegrees (Variables|Default|GetPhysHook) "0, 0, 0" false "None")
        (bind _returnvalue_6 (Physics|GetPhysicsLinearVelocity (Variables|/Script/Engine.Character|GetCapsuleComponent (Variables|Default|GetHero)) "None"))
        (Physics|SetPhysicsLinearVelocity (Variables|Default|GetPhysHook) (* _returnvalue_6 (Math|Float|MapRangeClamped _returnvalue_5 1e+03 0.0 0.0 1.0)) false "None")
        (Physics|AddForce (Variables|Default|GetPhysHook) (* (Math|Vector|Distance(Vector) _returnvalue_4 _returnvalue_3) (Math|Vector|GetUnitDirection(Vector) _returnvalue_4 _returnvalue_3) 5e+04 (Utilities|Time|GetWorldDeltaSeconds)) "None" true)
        (if (Math|Float|NearlyEqual(Float) _returnvalue_5 0.0 5e+01) ; Reconnect Hook ?
          (Variables|Default|SetSurface%20Type "SurfaceType4")
          (Transformation|SetWorldLocation _physhook_3 (Transformation|GetWorldLocation (Variables|Default|GetHookBase)) false true)
          (Physics|SetSimulatePhysics _physhook_3 false)
          (Transformation|AttachComponentToComponent (Variables|Default|GetPhysHook) (Variables|Transformation|GetRootComponent) "Hook attachment" "SnapToTarget" "SnapToTarget" "SnapToTarget" true)
          (Rendering|SetVisibility (Variables|Default|GetCable) false false)
          (Utilities|Time|ClearandInvalidateTimerbyHandle (Variables|Default|GetLaunchHookTimer))
          (CallFunction|ResetHookDetection)
          (goto _label Reset))))))

(event Input|EnhancedActionEvents|EnhancedInputActionIA_E
  (params (ActionValue :type Boolean) (ElapsedSeconds :type Float%20%28double-precision%29) (TriggeredSeconds :type Float%20%28double-precision%29) (InputAction :type Input%20Action%20Object%20Reference :default "/Game/Input/Actions/IA_E.IA_E"))
  (bind _herocam (Variables|Default|GetHeroCam))
  (bind _herocam_2 (Variables|Default|GetHeroCam))
  (bind _returnvalue (Transformation|GetWorldTransform _herocam))
  (bind _returnvalue_2 (Transformation|GetWorldLocation _herocam_2))
  (bind _returnvalue_3 (Transformation|GetWorldRotation _herocam_2))
  (bind _returnvalue_4 (Math|Vector|GetForwardVector _returnvalue_3))
  (bind _returnvalue_5 (* _returnvalue_4 1e+04))
  (bind _returnvalue_6 (+ _returnvalue_2 _returnvalue_5))
  (:Started
    (if (not (Utilities|Time|IsTimerActivebyHandle (Variables|Default|GetLaunchHookTimer)))
      (switch Utilities|FlowControl|Switch|SwitchonEPhysicalSurface (Variables|Default|GetSurface%20Type)
        (:SurfaceType3
          _)
        (:SurfaceType4
          _))
      (Utilities|FlowControl|Sequence
        (:then_0
          ;[0.15 0.15 0.15 0.5 50] General Setup
          (Rendering|SetVisibility (Variables|Default|GetCable) true false)
          (Variables|Default|SetSurface%20Type "SurfaceType4")
          (CallFunction|ToggleHookCollision true))
        (:then_1
          ;[0.15 0.15 0.15 0.5 50] Physically throw Hook
          (Transformation|DetachFromComponent (Variables|Default|GetPhysHook) "KeepWorld" "KeepWorld" "KeepWorld" true)
          (Transformation|SetWorldLocationAndRotation (Variables|Default|GetPhysHook) (.location _returnvalue) (.rotation _returnvalue) false false)
          (Transformation|AddLocalRotation (Variables|Default|GetPhysHook) "0.000000,-90.000000,0.000000" false false)
          (Physics|SetSimulatePhysics (Variables|Default|GetPhysHook) true)
          (Class|PrimitiveComponent|SetPhysicsAngularVelocityinDegrees (Variables|Default|GetPhysHook) "0, 0, 0" false "None")
          (Physics|SetPhysicsLinearVelocity (Variables|Default|GetPhysHook) "0, 0, 0" false "None")
          (bind (_outhit _returnvalue_7) (Collision|LineTraceByChannel _returnvalue_2 _returnvalue_6 "TraceTypeQuery1" false (Utilities|Array|MakeArray (Variables|Default|GetHero)) "None"))
          (bind _tossvelocity (Class|GameplayStatics|BlueprintSuggestProjectileVelocity (Transformation|GetWorldLocation (Variables|Default|GetPhysHook)) (Math|Vector|SelectVector (.ImpactPoint (Collision|BreakHitResult _outhit)) _returnvalue_6 _returnvalue_7) 5e+04 0.0 "DoNotTrace" 0.0 false false false))
          (Physics|AddImpulse (Variables|Default|GetPhysHook) _tossvelocity "None" false))
        (:then_2
          ;[0.15 0.15 0.15 0.5 50] Check for Hook exceeding max travel time
          (Variables|Default|SetHookRevoveryDelay 0.0)
          (bind _returnvalue_8 (Utilities|Time|SetTimerbyEvent (delegate Custom|CheckSurface) 0.001 true true))
          (Variables|Default|SetLaunchHookTimer _returnvalue_8))))))

(event Input|EnhancedActionEvents|EnhancedInputActionIA_LeftClick
  (params (ActionValue :type Boolean) (ElapsedSeconds :type Float%20%28double-precision%29) (TriggeredSeconds :type Float%20%28double-precision%29) (InputAction :type Input%20Action%20Object%20Reference :default "/Game/Input/Actions/IA_LeftClick.IA_LeftClick"))
  (bind _returnvalue (Components|GetOwner))
  (bind _hero (Variables|Default|GetHero))
  (bind _charactermovement (Variables|/Script/Engine.Character|GetCharacterMovement _hero))
  (:Triggered
    (switch Utilities|FlowControl|Switch|SwitchonEPhysicalSurface (Variables|Default|GetSurface%20Type)
      (:SurfaceType_Default
        _)
      (:SurfaceType2
        _))
    ;[0.15 0.15 0.15 0.5 50] Move Character To Location
    (if (Class|NavMovementInterface|IsFlying _charactermovement)
      _
      (else
        (Pawn|Components|CharacterMovement|SetMovementMode _charactermovement "MOVE_Flying" 0)))
    (Physics|AddForce (Variables|/Script/Engine.Character|GetCharacterMovement (Variables|Default|GetHero)) (* (Math|Vector|Normalize (+ (Math|Vector|GetUnitDirection(Vector) (Transformation|GetActorLocation _returnvalue) (Transformation|GetWorldLocation (Variables|Default|GetPhysHook))) (* (* (Transformation|GetActorRightVector _returnvalue) (.x (Variables|Default|GetAxis_Move))) 0.15))) 2.5e+05)))
  (:Started
    (switch Utilities|FlowControl|Switch|SwitchonEPhysicalSurface (Variables|Default|GetSurface%20Type)))
  (:Canceled
    (switch Utilities|FlowControl|Switch|SwitchonEPhysicalSurface (Variables|Default|GetSurface%20Type) :!label _label
      (:SurfaceType_Default
        _)
      (:SurfaceType1
        _)
      (:SurfaceType2
        _))
    (Pawn|Components|CharacterMovement|SetMovementMode (Variables|/Script/Engine.Character|GetCharacterMovement (Variables|Default|GetHero)) "MOVE_Falling" 0)
    (Physics|SetSimulatePhysics (Variables|Default|GetPhysHook) true)
    ;[0.15 0.15 0.15 0.5 50] Check for Hook exceeding max travel time
    (Variables|Default|SetHookRevoveryDelay 1.0)
    (bind _returnvalue_2 (Utilities|Time|SetTimerbyEvent (delegate Custom|CheckSurface) 0.001 true true))
    (Variables|Default|SetLaunchHookTimer _returnvalue_2))
  (:Completed
    (goto _label)))

(event Input|EnhancedActionEvents|EnhancedInputActionIA_MouseLook
  (params (ActionValue :type Vector%202D%20Structure) (ElapsedSeconds :type Float%20%28double-precision%29) (TriggeredSeconds :type Float%20%28double-precision%29) (InputAction :type Input%20Action%20Object%20Reference :default "/Game/Input/Actions/IA_MouseLook.IA_MouseLook"))
  (Variables|Default|SetAxis_Move (Math|Vector2D|MakeVector2D (.x ActionValue) (.y ActionValue))))

(event Input|EnhancedActionEvents|EnhancedInputActionIA_RightClick
  (params (ActionValue :type Boolean) (ElapsedSeconds :type Float%20%28double-precision%29) (TriggeredSeconds :type Float%20%28double-precision%29) (InputAction :type Input%20Action%20Object%20Reference :default "/Game/Input/Actions/IA_RightClick.IA_RightClick"))
  (:Started
    (switch Utilities|FlowControl|Switch|SwitchonEPhysicalSurface (Variables|Default|GetSurface%20Type)
      (:SurfaceType_Default
        _)
      (:SurfaceType1
        _)
      (:SurfaceType2
        _))
    (Physics|SetSimulatePhysics (Variables|Default|GetPhysHook) true)
    ;[0.15 0.15 0.15 0.5 50] Check for Hook exceeding max travel time
    (Variables|Default|SetHookRevoveryDelay 1.0)
    (bind _returnvalue (Utilities|Time|SetTimerbyEvent (delegate Custom|CheckSurface) 0.001 true true))
    (Variables|Default|SetLaunchHookTimer _returnvalue)))

(fn ConstructionScript)

(fn ToggleHookCollision
  (params (ON%20? :type Boolean))
  (if ON%20?
    (Collision|SetCollisionEnabled (Variables|Default|GetPhysHook) "QueryAndPhysics")
    (else
      (Collision|SetCollisionEnabled (Variables|Default|GetPhysHook) "NoCollision"))))