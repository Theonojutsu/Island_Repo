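; Projectile hook actor for a hook weapon that flies until it strikes something other than its Instigator.
; EnableProjectile toggles the projectile movement component and physics simulation on the hook's collision component together.
; The first valid hit, gated by DoOnce, teleports the collision component to the impact point and disables both, freezing the hook in place.
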(event OnComponentHit(HookCollision)
  (params (HitComponent :type Primitive%20Component%20Object%20Reference) (OtherActor :type Actor%20Object%20Reference) (OtherComp :type Primitive%20Component%20Object%20Reference) (NormalImpulse :type Vector :default "0, 0, 0") (Hit :type Hit%20Result%20Structure%20%28by%20ref%29))
  (if (!= OtherActor (Variables|Actor|GetInstigator))
    (Utilities|FlowControl|DoOnce false
      (:Completed
        (Transformation|SetWorldLocation (Variables|Default|GetHookCollision) (.ImpactPoint (Collision|BreakHitResult Hit)) false true)
        (CallFunction|EnableProjectile false)))))

(event Custom|EnableProjectile
  (params (True :type Boolean))
  (Components|Activation|SetActive (Variables|Default|GetProjectileMovement) True false)
  (Physics|SetSimulatePhysics (Variables|Default|GetHookCollision) True))

(fn ConstructionScript)