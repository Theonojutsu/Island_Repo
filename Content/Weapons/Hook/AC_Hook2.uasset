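; Actor component that sets up a hand-held grappling hook on its owning Character, apparently an unfinished version.
; On BeginPlay it caches the character and camera, builds hook base and hook meshes on the left hand socket, links them with a cable, and spawns a projectile hook actor.
; Move input is stored, while launch input checks a timer and surface type but its visible branches perform no action yet.
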(event Input|EnhancedActionEvents|EnhancedInputActionIA_Move
  (params (ActionValue :type Vector%202D%20Structure) (ElapsedSeconds :type Float%20%28double-precision%29) (TriggeredSeconds :type Float%20%28double-precision%29) (InputAction :type Input%20Action%20Object%20Reference :default "/Game/Input/Actions/IA_Move.IA_Move"))
  (Variables|Default|SetAxis_Move ActionValue))

(event Input|EnhancedActionEvents|EnhancedInputActionIA_Hook_Launch
  (params (ActionValue :type Boolean) (ElapsedSeconds :type Float%20%28double-precision%29) (TriggeredSeconds :type Float%20%28double-precision%29) (InputAction :type Input%20Action%20Object%20Reference :default "/Game/Input/Actions/IA_Hook_Launch.IA_Hook_Launch"))
  (:Started
    (if (not (Utilities|Time|IsTimerActivebyHandle (Variables|Default|GetLaunchHookTimer)))
      (switch Utilities|FlowControl|Switch|SwitchonEPhysicalSurface (Variables|Default|GetSurface%20Type)
        (:SurfaceType3
          _)
        (:SurfaceType4
          _))
      (Utilities|FlowControl|Sequence))))

(event EventBeginPlay
  (Utilities|FlowControl|Sequence
    (:then_0
      (bind _ascharacter (Utilities|Casting|CastToCharacter (Components|GetOwner)))
      (Variables|Default|SetHero _ascharacter))
    (:then_1
      (Utilities|IsValid (Actor|GetComponentbyClass (Variables|Default|GetHero) "/Script/Engine.CameraComponent")
        (:Is%20Valid
          (Variables|Default|SetHero_Cam (Actor|GetComponentbyClass (Variables|Default|GetHero) "/Script/Engine.CameraComponent")))))
    (:then_2
      (bind _returnvalue (Game|AddComponentbyClass (Variables|Default|GetHero) "/Script/Engine.StaticMeshComponent" false)) ; Base
      (bind _output_get (Variables|Default|SetHook_Base _returnvalue))
      (Components|StaticMesh|SetStaticMesh _output_get "/Game/Weapons/Hook/Models/SM_HookBase.SM_HookBase")
      (Transformation|AttachComponentToComponent _output_get (Variables|/Script/Engine.Character|GetMesh (Variables|Default|GetHero)) "HandGrip_L" "SnapToTarget" "SnapToTarget" "KeepWorld" true))
    (:then_3
      (bind _returnvalue_2 (Game|AddComponentbyClass (Variables|Default|GetHero) "/Script/Engine.StaticMeshComponent" false)) ; Hook
      (bind _output_get_2 (Variables|Components|SetHook _returnvalue_2))
      (Components|StaticMesh|SetStaticMesh _output_get_2 "/Game/Weapons/Hook/Models/SM_Hook.SM_Hook")
      (Transformation|AttachComponentToComponent _output_get_2 _output_get "HookAttachment" "SnapToTarget" "SnapToTarget" "KeepWorld" true))
    (:then_4
      (bind _returnvalue_3 (Game|AddComponentbyClass (Variables|Default|GetHero) "/Script/CableComponent.CableComponent" false))
      (Rendering|Material|SetMaterial _returnvalue_3 0 "/Game/Weapons/Hook/Materials/M_Rope.M_Rope")
      (Variables|/Script/CableComponent.CableComponent|SetEndLocation _returnvalue_3 "0, 0, 0")
      (Transformation|AttachComponentToComponent _returnvalue_3 (Variables|Components|GetHook) "CableAttachment" "SnapToTarget" "SnapToTarget" "KeepWorld" false)
      (Class|CableComponent|SetAttachEndtoComponent _returnvalue_3 (Variables|Default|GetHook_Base) "HookBase"))
    (:then_5
      (Game|SpawnActorfromClass "/Game/Weapons/Hook/BP_ProjectileHook.BP_ProjectileHook_C" (Transformation|GetActorTransform (Variables|Default|GetHero)) "AlwaysSpawn" "MultiplyWithRoot" (Variables|Default|GetHero) (Variables|Default|GetHero)))))