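; Actor component giving its owning Character a physics grappling hook that fires, sticks and reels the hero in.
; IA_E launches a spawned BP_HookArm's hook using camera trace and suggested projectile velocity; hits stick by physical surface type or on other characters.
; A looping timer recalls missed hooks with force until they reattach.
; Left click pulls the flying hero with side steering and wider FOV; release or right click recalls the hook.
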(event Custom|UpdateFOV
  (params (Increase? :type Boolean))
  (if Increase?
    (bind _alpha (Utilities|ComponentTimeline 4.0 "/Game/Libraries/Data/Curves/C_Linear.C_Linear" :!label _label)
      (:Update
        (Camera|SetFieldOfView (Variables|Default|GetHeroCam) (Math|Float|Lerp 9e+01 1.1e+02 _alpha))))
    (else
      (goto _label Reverse))))

(event Custom|ToggleHookCollision
  (params (ON%20? :type Boolean))
  (bind _hookarm (Variables|Default|GetHookArm))
  (bind _hookarm_2 (Variables|Default|GetHookArm))
  (bind _physhook (Variables|/Game/Weapons/Hook/BP_HookArm.BP_HookArm_C|GetPhysHook _hookarm_2))
  (bind _physhook_2 (Variables|/Game/Weapons/Hook/BP_HookArm.BP_HookArm_C|GetPhysHook _hookarm))
  (if ON%20?
    (Collision|BindEventtoOnComponentHit _physhook_2 (EventDispatchers|CreateEvent :!event Custom|OnHookHit))
    (Collision|BindEventtoOnComponentBeginOverlap _physhook_2 (EventDispatchers|CreateEvent :!event Custom|OnOverlapPlayers))
    (Collision|SetCollisionResponsetoAllChannels _physhook "ECR_Block")
    (Collision|SetCollisionResponsetoChannel _physhook "ECC_Visibility" "ECR_Ignore")
    (Collision|SetCollisionResponsetoChannel _physhook "ECC_Camera" "ECR_Ignore")
    (Collision|SetCollisionResponsetoChannel _physhook "ECC_Pawn" "ECR_Overlap")
    (else
      (Collision|UnbindEventfromOnComponentHit _physhook_2 (EventDispatchers|CreateEvent :!event Custom|OnHookHit))
      (Collision|UnbindEventfromOnComponentBeginOverlap _physhook_2 (EventDispatchers|CreateEvent :!event Custom|OnOverlapPlayers))
      (Collision|SetCollisionResponsetoAllChannels _physhook "ECR_Ignore"))))

(event Custom|OnOverlapPlayers
  (params (OverlappedComponent :type Primitive%20Component%20Object%20Reference) (OtherActor :type Actor%20Object%20Reference) (OtherComp :type Primitive%20Component%20Object%20Reference) (OtherBodyIndex :type Integer) (bFromSweep :type Boolean) (SweepResult :type Hit%20Result%20Structure%20%28by%20ref%29))
  (bind _hookarm (Variables|Default|GetHookArm))
  (bind _physhook (Variables|/Game/Weapons/Hook/BP_HookArm.BP_HookArm_C|GetPhysHook _hookarm))
  ;[0.15 0.15 0.15 0.5 50] Stick to surface
  (if (!= OtherActor (Variables|Default|GetHero))
    (Utilities|Casting|CastToCharacter OtherActor)
    (Variables|Default|SetSurface%20Type "SurfaceType1")
    (Transformation|SetWorldLocation _physhook (Transformation|GetWorldLocation _physhook) false true)
    (Physics|SetSimulatePhysics (Variables|/Game/Weapons/Hook/BP_HookArm.BP_HookArm_C|GetPhysHook (Variables|Default|GetHookArm)) false)
    (Utilities|Time|ClearandInvalidateTimerbyHandle (Variables|Default|GetLaunchHookTimer))
    (Camera|PlayWorldCameraShake "/Game/FirstPerson/Camera/CS_ShakeToSurface.CS_ShakeToSurface_C" (Transformation|GetActorLocation (Variables|Default|GetHero)) 0.0 5e+02)
    (CallFunction|ToggleHookCollision false)))

(event Custom|CheckSurface
  (bind _hookarm (Variables|Default|GetHookArm))
  (bind _hookarm_2 (Variables|Default|GetHookArm))
  (bind _hookarm_3 (Variables|Default|GetHookArm))
  (bind _hookarm_4 (Variables|Default|GetHookArm))
  (bind _hookarm_5 (Variables|Default|GetHookArm))
  (bind _physhook (Variables|/Game/Weapons/Hook/BP_HookArm.BP_HookArm_C|GetPhysHook _hookarm_5))
  (bind _hookbase (Variables|/Game/Weapons/Hook/BP_HookArm.BP_HookArm_C|GetHookBase _hookarm))
  (bind _physhook_2 (Variables|/Game/Weapons/Hook/BP_HookArm.BP_HookArm_C|GetPhysHook _hookarm_2))
  (bind _hookbase_2 (Variables|/Game/Weapons/Hook/BP_HookArm.BP_HookArm_C|GetHookBase _hookarm_3))
  (bind _physhook_3 (Variables|/Game/Weapons/Hook/BP_HookArm.BP_HookArm_C|GetPhysHook _hookarm_4))
  (bind _returnvalue (Transformation|GetWorldLocation _physhook))
  (bind _returnvalue_2 (Transformation|GetWorldLocation _hookbase))
  (bind _returnvalue_3 (Transformation|GetWorldLocation _hookbase_2))
  (bind _returnvalue_4 (Transformation|GetWorldLocation _physhook_2))
  (bind _returnvalue_5 (Math|Vector|Distance(Vector) _returnvalue _returnvalue_2))
  ;[0.15 0.15 0.15 0.5 50] Check for Hook exceeding max travel time
  (bind _output_get (Variables|Default|SetHookRevoveryDelay (+ (Utilities|Time|GetWorldDeltaSeconds) (stale _output_get))))
  (if (> _output_get 1.0) ; Hook's max travel time reached ?
    ;[0.15 0.15 0.15 0.5 50] Recall Hook
    (Utilities|FlowControl|Sequence
      (:then_0
        (Utilities|FlowControl|DoOnce false :!label _label
          (:Completed
            (CallFunction|ToggleHookCollision false))))
      (:then_1
        (Class|PrimitiveComponent|SetPhysicsAngularVelocityinDegrees (Variables|/Game/Weapons/Hook/BP_HookArm.BP_HookArm_C|GetPhysHook (Variables|Default|GetHookArm)) "0, 0, 0" false "None")
        (bind _returnvalue_6 (Physics|GetPhysicsLinearVelocity (Variables|/Script/Engine.Character|GetCapsuleComponent (Variables|Default|GetHero)) "None"))
        (Physics|SetPhysicsLinearVelocity (Variables|/Game/Weapons/Hook/BP_HookArm.BP_HookArm_C|GetPhysHook (Variables|Default|GetHookArm)) (* _returnvalue_6 (Math|Float|MapRangeClamped _returnvalue_5 1e+03 0.0 0.0 1.0)) false "None")
        (Physics|AddForce (Variables|/Game/Weapons/Hook/BP_HookArm.BP_HookArm_C|GetPhysHook (Variables|Default|GetHookArm)) (* (Math|Vector|Distance(Vector) _returnvalue_4 _returnvalue_3) (Math|Vector|GetUnitDirection(Vector) _returnvalue_4 _returnvalue_3) 5e+04 (Utilities|Time|GetWorldDeltaSeconds)) "None" true)
        (if (Math|Float|NearlyEqual(Float) _returnvalue_5 0.0 5e+01) ; Reconnect Hook ?
          (Variables|Default|SetSurface%20Type "SurfaceType4")
          (Transformation|SetWorldLocation _physhook_3 (Transformation|GetWorldLocation (Variables|/Game/Weapons/Hook/BP_HookArm.BP_HookArm_C|GetHookBase (Variables|Default|GetHookArm))) false true)
          (Physics|SetSimulatePhysics _physhook_3 false)
          (Transformation|AttachComponentToComponent (Variables|/Game/Weapons/Hook/BP_HookArm.BP_HookArm_C|GetPhysHook (Variables|Default|GetHookArm)) (Variables|/Script/Engine.Actor|GetRootComponent (Variables|Default|GetHookArm)) "ProjectileAttachment" "SnapToTarget" "SnapToTarget" "SnapToTarget" true)
          (Rendering|SetVisibility (Variables|/Game/Weapons/Hook/BP_HookArm.BP_HookArm_C|GetCable (Variables|Default|GetHookArm)) false false)
          (Utilities|Time|ClearandInvalidateTimerbyHandle (Variables|Default|GetLaunchHookTimer))
          (goto _label Reset))))))

(event Custom|OnHookHit
  (params (HitComponent :type Primitive%20Component%20Object%20Reference) (OtherActor :type Actor%20Object%20Reference) (OtherComp :type Primitive%20Component%20Object%20Reference) (NormalImpulse :type Vector) (Hit :type Hit%20Result%20Structure%20%28by%20ref%29))
  (bind _hookarm (Variables|Default|GetHookArm))
  (bind _physhook (Variables|/Game/Weapons/Hook/BP_HookArm.BP_HookArm_C|GetPhysHook _hookarm))
  ;[0.15 0.15 0.15 0.5 50] Stick to surface
  (bind _output_get (Variables|Default|SetSurface%20Type (Variables|/Script/PhysicsCore.PhysicalMaterial|GetSurfaceType (.PhysMat (Collision|BreakHitResult Hit)))))
  (if (and (Utilities|Enum|NotEqual(Enum) _output_get "SurfaceType4") (Utilities|Enum|NotEqual(Enum) _output_get "SurfaceType3"))
    (Transformation|SetWorldLocation _physhook (Transformation|GetWorldLocation _physhook) false true)
    (Physics|SetSimulatePhysics (Variables|/Game/Weapons/Hook/BP_HookArm.BP_HookArm_C|GetPhysHook (Variables|Default|GetHookArm)) false)
    (Utilities|Time|ClearandInvalidateTimerbyHandle (Variables|Default|GetLaunchHookTimer))
    (Camera|PlayWorldCameraShake "/Game/FirstPerson/Camera/CS_ShakeToSurface.CS_ShakeToSurface_C" (Transformation|GetActorLocation (Variables|Default|GetHero)) 0.0 5e+02)
    (CallFunction|ToggleHookCollision false)))

(event Input|EnhancedActionEvents|EnhancedInputActionIA_Move
  (params (ActionValue :type Vector%202D%20Structure) (ElapsedSeconds :type Float%20%28double-precision%29) (TriggeredSeconds :type Float%20%28double-precision%29) (InputAction :type Input%20Action%20Object%20Reference :default "/Game/Input/Actions/IA_Move.IA_Move"))
  (Variables|Default|SetAxis_Move (Math|Vector2D|MakeVector2D (.x ActionValue) (.y ActionValue))))

(event Input|EnhancedActionEvents|EnhancedInputActionIA_E
  (params (ActionValue :type Boolean) (ElapsedSeconds :type Float%20%28double-precision%29) (TriggeredSeconds :type Float%20%28double-precision%29) (InputAction :type Input%20Action%20Object%20Reference :default "/Game/Input/Actions/IA_E.IA_E"))
  (bind _returnvalue (Math|Float|MakeLiteralFloat 1e+04))
  (bind _herocam (Variables|Default|GetHeroCam))
  (bind _hookarm (Variables|Default|GetHookArm))
  (bind _herocam_2 (Variables|Default|GetHeroCam))
  (bind _hookarm_2 (Variables|Default|GetHookArm))
  (bind _returnvalue_2 (Transformation|GetWorldLocation _herocam_2))
  (bind _returnvalue_3 (Transformation|GetWorldRotation _herocam_2))
  (bind _returnvalue_4 (Transformation|GetWorldTransform _herocam))
  (bind _physhook (Variables|/Game/Weapons/Hook/BP_HookArm.BP_HookArm_C|GetPhysHook _hookarm))
  (bind _physhook_2 (Variables|/Game/Weapons/Hook/BP_HookArm.BP_HookArm_C|GetPhysHook _hookarm_2))
  (bind _returnvalue_5 (Transformation|GetWorldLocation _physhook))
  (bind _returnvalue_6 (Math|Vector|GetForwardVector _returnvalue_3))
  (bind _returnvalue_7 (* _returnvalue_6 _returnvalue))
  (bind _returnvalue_8 (+ _returnvalue_2 _returnvalue_7))
  (:Started
    (if (not (Utilities|Time|IsTimerActivebyHandle (Variables|Default|GetLaunchHookTimer)))
      (switch Utilities|FlowControl|Switch|SwitchonEPhysicalSurface (Variables|Default|GetSurface%20Type)
        (:SurfaceType3
          _)
        (:SurfaceType4
          _))
      (Utilities|FlowControl|Sequence
        (:then_0
          ;[0.15 0.15 0.15 0.5 50] General Setup
          (Rendering|SetVisibility (Variables|/Game/Weapons/Hook/BP_HookArm.BP_HookArm_C|GetCable (Variables|Default|GetHookArm)) true false)
          (Variables|Default|SetSurface%20Type "SurfaceType4"))
        (:then_1
          ;[0.15 0.15 0.15 0.5 50] Physically throw Hook
          (CallFunction|ToggleHookCollision true)
          (Transformation|SetWorldLocationAndRotation (Variables|/Game/Weapons/Hook/BP_HookArm.BP_HookArm_C|GetPhysHook (Variables|Default|GetHookArm)) (.location _returnvalue_4) (.rotation _returnvalue_4) false false)
          (Transformation|AddLocalRotation (Variables|/Game/Weapons/Hook/BP_HookArm.BP_HookArm_C|GetPhysHook (Variables|Default|GetHookArm)) "0.000000,-90.000000,0.000000" false false)
          (Physics|SetSimulatePhysics _physhook_2 true)
          (Class|PrimitiveComponent|SetPhysicsAngularVelocityinDegrees _physhook_2 "0, 0, 0" false "None")
          (Physics|SetPhysicsLinearVelocity _physhook_2 "0, 0, 0" false "None")
          (bind (_outhit _returnvalue_9) (Collision|LineTraceByChannel _returnvalue_2 _returnvalue_8 "TraceTypeQuery1" false (Utilities|Array|MakeArray (Variables|Default|GetHero)) "None"))
          (bind _tossvelocity (Class|GameplayStatics|BlueprintSuggestProjectileVelocity _returnvalue_5 (+ (Math|Vector|MakeVector 0.0 0.0 (Math|Float|MapRangeClamped (Math|Vector|Distance(Vector) _returnvalue_5 (Math|Vector|SelectVector (.ImpactPoint (Collision|BreakHitResult _outhit)) _returnvalue_8 _returnvalue_9)) 1.5e+03 _returnvalue 0.0 6e+02)) (Math|Vector|SelectVector (.ImpactPoint (Collision|BreakHitResult _outhit)) _returnvalue_8 _returnvalue_9)) 7.5e+04 0.0 "DoNotTrace" (Variables|/Script/Engine.SphereComponent|GetSphereRadius _physhook) false false false))
          (Physics|AddImpulse (Variables|/Game/Weapons/Hook/BP_HookArm.BP_HookArm_C|GetPhysHook (Variables|Default|GetHookArm)) _tossvelocity "None" false))
        (:then_2
          ;[0.15 0.15 0.15 0.5 50] Check for Hook exceeding max travel time
          (Variables|Default|SetHookRevoveryDelay 0.0)
          (bind _returnvalue_10 (Utilities|Time|SetTimerbyEvent (delegate Custom|CheckSurface) 0.001 true true))
          (Variables|Default|SetLaunchHookTimer _returnvalue_10))))))

(event Input|EnhancedActionEvents|EnhancedInputActionIA_RightClick
  (params (ActionValue :type Boolean) (ElapsedSeconds :type Float%20%28double-precision%29) (TriggeredSeconds :type Float%20%28double-precision%29) (InputAction :type Input%20Action%20Object%20Reference :default "/Game/Input/Actions/IA_RightClick.IA_RightClick"))
  (:Started
    (switch Utilities|FlowControl|Switch|SwitchonEPhysicalSurface (Variables|Default|GetSurface%20Type)
      (:SurfaceType_Default
        _)
      (:SurfaceType1
        _)
      (:SurfaceType2
        _))
    (Camera|PlayWorldCameraShake "/Game/FirstPerson/Camera/CS_ShakeToSurface.CS_ShakeToSurface_C" (Transformation|GetActorLocation (Variables|Default|GetHero)) 0.0 5e+02)
    (Physics|SetSimulatePhysics (Variables|/Game/Weapons/Hook/BP_HookArm.BP_HookArm_C|GetPhysHook (Variables|Default|GetHookArm)) true)
    ;[0.15 0.15 0.15 0.5 50] Check for Hook exceeding max travel time
    (Variables|Default|SetHookRevoveryDelay 1.0)
    (bind _returnvalue (Utilities|Time|SetTimerbyEvent (delegate Custom|CheckSurface) 0.001 true true))
    (Variables|Default|SetLaunchHookTimer _returnvalue)))

(event Input|EnhancedActionEvents|EnhancedInputActionIA_LeftClick
  (params (ActionValue :type Boolean) (ElapsedSeconds :type Float%20%28double-precision%29) (TriggeredSeconds :type Float%20%28double-precision%29) (InputAction :type Input%20Action%20Object%20Reference :default "/Game/Input/Actions/IA_LeftClick.IA_LeftClick"))
  (bind _returnvalue (Components|GetOwner))
  (bind _hero (Variables|Default|GetHero))
  (bind _charactermovement (Variables|/Script/Engine.Character|GetCharacterMovement _hero))
  (:Triggered
    (switch Utilities|FlowControl|Switch|SwitchonEPhysicalSurface (Variables|Default|GetSurface%20Type)
      (:SurfaceType_Default
        _)
      (:SurfaceType2
        _))
    ;[0.15 0.15 0.15 0.5 50] Move Character To Location
    (if (Class|NavMovementInterface|IsFlying _charactermovement)
      _
      (else
        (Pawn|Components|CharacterMovement|SetMovementMode _charactermovement "MOVE_Flying" 0)))
    (Physics|AddForce (Variables|/Script/Engine.Character|GetCharacterMovement (Variables|Default|GetHero)) (* (Math|Vector|Normalize (+ (Math|Vector|GetUnitDirection(Vector) (Transformation|GetActorLocation _returnvalue) (Transformation|GetWorldLocation (Variables|/Game/Weapons/Hook/BP_HookArm.BP_HookArm_C|GetPhysHook (Variables|Default|GetHookArm)))) (* (* (Transformation|GetActorRightVector _returnvalue) (.x (Variables|Default|GetAxis_Move))) 0.15))) 2.5e+05)))
  (:Started
    (switch Utilities|FlowControl|Switch|SwitchonEPhysicalSurface (Variables|Default|GetSurface%20Type)
      (:SurfaceType_Default
        _)
      (:SurfaceType2
        _))
    (CallFunction|UpdateFOV true))
  (:Canceled
    (switch Utilities|FlowControl|Switch|SwitchonEPhysicalSurface (Variables|Default|GetSurface%20Type) :!label _label
      (:SurfaceType_Default
        _)
      (:SurfaceType1
        _)
      (:SurfaceType2
        _))
    (CallFunction|UpdateFOV false)
    (Pawn|Components|CharacterMovement|SetMovementMode (Variables|/Script/Engine.Character|GetCharacterMovement (Variables|Default|GetHero)) "MOVE_Falling" 0)
    (Camera|PlayWorldCameraShake "/Game/FirstPerson/Camera/CS_ShakeToSurface.CS_ShakeToSurface_C" (Transformation|GetActorLocation (Variables|Default|GetHero)) 0.0 5e+02)
    (Physics|SetSimulatePhysics (Variables|/Game/Weapons/Hook/BP_HookArm.BP_HookArm_C|GetPhysHook (Variables|Default|GetHookArm)) true)
    ;[0.15 0.15 0.15 0.5 50] Check for Hook exceeding max travel time
    (Variables|Default|SetHookRevoveryDelay 1.0)
    (bind _returnvalue_2 (Utilities|Time|SetTimerbyEvent (delegate Custom|CheckSurface) 0.001 true true))
    (Variables|Default|SetLaunchHookTimer _returnvalue_2))
  (:Completed
    (goto _label)))

(event EventBeginPlay
  (Utilities|FlowControl|Sequence
    (:then_0
      (Variables|Default|GetHero
        (:then)
        (:else
          (bind _ascharacter (Utilities|Casting|CastToCharacter (Components|GetOwner)))
          (bind _output_get (Variables|Default|SetHero _ascharacter))
          (bind _returnvalue (Game|SpawnActorfromClass "/Game/Weapons/Hook/BP_HookArm.BP_HookArm_C" (Math|Transform|MakeTransform "0, 0, 0" "0, 0, 0" "1.000000,1.000000,1.000000") "Undefined" "MultiplyWithRoot" 0 0))
          (Default|AttachSelftoHero _returnvalue _output_get)
          (Variables|Default|SetHookArm _returnvalue))))
    (:then_1
      (Variables|Default|SetHeroCam (Actor|GetComponentbyClass (Variables|Default|GetHero) "/Script/Engine.CameraComponent")))))

(fn NewFunction
  (params (StartPos :type Vector) (LaunchVelocity :type Vector) (ProjectileRadius :type Float%20%28single-precision%29))
  (bind _outpathpositions (Class|GameplayStatics|BlueprintPredictProjectilePathbyObjectType StartPos LaunchVelocity true ProjectileRadius (Utilities|Array|MakeArray "ObjectTypeQuery5") false 0 "None" 5.0 5.0 1.0))
  (for _array_element _outpathpositions
    (if (>= (.Z (Math|Vector|BreakVector _array_element)) (LocalVariables|GetNewLocalVar_1))
      (LocalVariables|SetNewLocalVar_1 (.Z (Math|Vector|BreakVector _array_element)))
      (LocalVariables|SetNewLocalVar_2 _array_element)))
  (return (LocalVariables|GetNewLocalVar_2) (Utilities|Array|Get(acopy) _outpathpositions (Utilities|Array|LastIndex _outpathpositions)) StartPos))