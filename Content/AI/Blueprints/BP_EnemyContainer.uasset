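; BP_EnemyContainer draws a group of enemies as instances of one InstancedStaticMesh and moves them over time.
; The construction script adds EnemyCount instances spaced along local Y and stores their indices in InstancesInt.
; Tick sets each instance's world X and Y from real time scaled by array position, so they slide diagonally at increasing speeds.
; Pathfinding and distance nodes are present but never run.
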(event EventTick
  (params (DeltaSeconds :type Float%20%28single-precision%29))
  (for (_array_element _array_index) (Variables|Default|GetInstancesInt)
    (Components|InstancedStaticMesh|UpdateInstanceTransform (Variables|Default|GetInstancedStaticMesh) _array_element (Math|Transform|MakeTransform (Math|Vector|MakeVector (* (+ _array_index 1) (* (Utilities|Time|GetRealTimeSeconds) 1e+02)) (* (+ _array_index 1) (* (Utilities|Time|GetRealTimeSeconds) 1e+02)) 0.0) "0, 0, 0" "1.000000,1.000000,1.000000") true false false)))

(fn ConstructionScript
  (for _index (range 0 (- (Variables|Default|GetEnemyCount) 1))
    (bind _returnvalue (Components|InstancedStaticMesh|AddInstance (Variables|Default|GetInstancedStaticMesh) (Math|Transform|MakeTransform (Math|Vector|MakeVector 0.0 (Math|Conversions|ToFloat(Integer) (* _index 100)) 0.0)) false))
    (Utilities|Array|AddUnique (Variables|Default|GetInstancesInt) _returnvalue)))